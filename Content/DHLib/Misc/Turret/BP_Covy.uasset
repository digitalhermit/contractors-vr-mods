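; BP_Covy is an auto-targeting defensive turret that shoots at nearby pawns.
; Each tick the authority picks the closest pawn in its sphere scanner (the line-of-sight result goes unused), then MCProcessTarget feeds target and tuning to the Covy_Defender AnimBP.
; When the AnimBP signals fire, the authority rate-limits shots by ShotDelay, launching a damage projectile along the turret's aim with a matching particle effect and multicast sound.
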(event `self.ReceiveBeginPlay`
  ;[1 1 1] Initialization
  (set `self.LastFireTime` 0.0))

(event `self.ReceiveTick`
  (params (DeltaSeconds :type "Float (single-precision)"))
  ;[1 1 1] Keep Turrent Animation State and Firing in Sync across all Clients
  (`/Engine/EditorBlueprintResources/ActorMacros.Switch Has Authority`
    (:`Authority`
      (`self.FindBestTarget`)
      (`self.MC Process Target`))))

(event `MC Process Target`
  (bind _target (`self.Target`))
  (bind _returnvalue (`SkeletalMeshComponent.GetAnimInstance` (`self.Turret`)))
  ;[1 1 1] Keep Turrent Animation State and Firing in Sync across all Clients
  (`/Engine/EditorBlueprintResources/StandardMacros.IsValid` _target
    (:`Is Valid`
      (bind _ascovy_defender_anim_bp (cast `/Game/DHLib/Misc/Turret/Covy_Defender_AnimBP` _returnvalue))
      (`self.ConfigureAnimBP` _ascovy_defender_anim_bp)
      (`/Game/DHLib/Misc/Turret/Covy_Defender_AnimBP.TargetAcquired` _ascovy_defender_anim_bp _target)
      (`/Engine/EditorBlueprintResources/ActorMacros.Switch Has Authority`
        (:`Authority`
          (if (`/Game/DHLib/Misc/Turret/Covy_Defender_AnimBP.fire_at_target` _ascovy_defender_anim_bp)
            (`self.MaybeFire`)))))
    (:`Is Not Valid`
      (bind _ascovy_defender_anim_bp_2 (cast `/Game/DHLib/Misc/Turret/Covy_Defender_AnimBP` _returnvalue))
      (`self.ConfigureAnimBP` _ascovy_defender_anim_bp_2)
      (`/Game/DHLib/Misc/Turret/Covy_Defender_AnimBP.TargetOutOfRange` _ascovy_defender_anim_bp_2))))

(event `SRVPlaySoundOnAll`
  (params (Audio :type "AudioComponent Object Reference"))
  ;[1 1 1] Sound to Server and then Multicast to All
  (`self.MCPlaySound` Audio))

(event `MCPlaySound`
  (params (Audio :type "AudioComponent Object Reference"))
  ;[1 1 1] Sound to Server and then Multicast to All
  (`ActorComponent.Activate` Audio false)
  (`AudioComponent.Play` Audio 0.0))

(event `FireParticleSystem`
  (params (Velocity :type "Vector Structure"))
  (bind _particleprojectile (`self.ParticleProjectile`))
  ;[1 1 1] Fire Particle System & Hidden Projectile (to support damage)
  (`ActorComponent.Activate` _particleprojectile false)
  (`NiagaraComponent.SetVariableVec3` _particleprojectile "Velocity" Velocity)
  (`NiagaraComponent.ResetSystem` _particleprojectile)
  (`self.MCPlaySound` (`self.TurretBlast`)))

(event `FireProjectile`
  (params (Transform :type "Transform Structure") (Velocity :type "Vector Structure"))
  ;[1 1 1] Fire Particle System & Hidden Projectile (to support damage)
  (bind _returnvalue (`|SpawnActorFromClass` "/Game/DHLib/Misc/Turret/CovyProjectile.CovyProjectile_C" Transform "AlwaysSpawn" "OverrideRootScale" null null))
  (`ProjectileMovementComponent.SetVelocityInLocalSpace` (`/Game/DHLib/Misc/Turret/CovyProjectile.ProjectileMovement` _returnvalue) Velocity)
  (set `/Game/DHLib/Misc/Turret/CovyProjectile.BaseDamage` (`self.BaseDamage`) _returnvalue)
  (set `/Game/DHLib/Misc/Turret/CovyProjectile.SourceTurret` self _returnvalue))

(fn `ConfigureAnimBP`
  (params (`Anim BP` :type "/Game/DHLib/Misc/Turret/Covy_Defender_AnimBP Object Reference"))
  (set `/Game/DHLib/Misc/Turret/Covy_Defender_AnimBP.muzzle_velocity` (`self.MuzzleVelocity`) `Anim BP`)
  (set `/Game/DHLib/Misc/Turret/Covy_Defender_AnimBP.aggressiveness` (`self.Aggressiveness`) `Anim BP`)
  (set `/Game/DHLib/Misc/Turret/Covy_Defender_AnimBP.scan_angle` (`self.ScanAngle`) `Anim BP`))

(fn `FindBestTarget`
  (locals (`BestDistance (local)` :type "Float (double-precision)") (`CurrentDistance (local)` :type "Float (double-precision)") (`BestTarget (local)` :type "Pawn Object Reference") (`CurrentTarget (local)` :type "Pawn Object Reference"))
  (bind _currenttarget__local_ (`local.CurrentTarget (local)`))
  (set `local.BestDistance (local)` (+ (`self.SensingRange`) 1.0))
  (for _array_element (`PrimitiveComponent.GetOverlappingActors` (`self.SphereScanner`) null)
    (bind _aspawn (cast `Pawn` _array_element))
    (bind _output_get (set `local.CurrentTarget (local)` _aspawn))
    (bind _output_get_2 (set `local.CurrentDistance (local)` (`self.GetDistanceTo` _output_get self)))
    (if (or (< _output_get_2 (`local.BestDistance (local)`)) (not (`KismetSystemLibrary.IsValid` (`local.BestTarget (local)`))))
      (`self.HasLineOfSight` (`SceneComponent.K2_GetComponentLocation` (`self.Turret`)) (`self.K2_GetActorLocation` _currenttarget__local_) (`|MakeArray` self _currenttarget__local_ :!type "Actor Object Reference"))
      (set `local.BestTarget (local)` (`local.CurrentTarget (local)`))
      (set `local.BestDistance (local)` (`local.CurrentDistance (local)`))))
  (set `self.Target` (`local.BestTarget (local)`)))

(fn `HasLineOfSight`
  (params (From :type "Vector Structure") (To :type "Vector Structure") (ActorsToIgnore :type "Array of Actor Object Reference (by ref)"))
  (returns (Result :type Boolean))
  (bind (_outhit _returnvalue) (`KismetSystemLibrary.LineTraceSingle` From To "TraceTypeQuery1" false ActorsToIgnore))
  (return (not _returnvalue)))

(fn `Initialize`
  (params (MuzzleVelocity :type "Float (double-precision)") (BaseDamage :type "Float (double-precision)") (ScanAngle :type "Float (double-precision)") (Aggressiveness :type "Float (double-precision)") (ShotDelay :type "Float (double-precision)"))
  (set `self.MuzzleVelocity` (`KismetMathLibrary.FClamp` MuzzleVelocity 100.0 20000.0))
  (set `self.BaseDamage` (`KismetMathLibrary.FClamp` BaseDamage 0.0 1000.0))
  (set `self.ScanAngle` (`KismetMathLibrary.FClamp` ScanAngle 0.0 180.0))
  (set `self.Aggressiveness` (`KismetMathLibrary.FClamp` Aggressiveness 1.0 100.0))
  (set `self.ShotDelay` (`KismetMathLibrary.FClamp` ShotDelay 0.1 300.0)))

(fn `MaybeFire`
  (bind _returnvalue (`KismetSystemLibrary.GetGameTimeInSeconds`))
  (bind _turret (`self.Turret`))
  (if (> (- _returnvalue (`self.LastFireTime`)) (`self.ShotDelay`))
    (set `self.LastFireTime` _returnvalue)
    (bind _ascovy_defender_anim_bp (cast `/Game/DHLib/Misc/Turret/Covy_Defender_AnimBP` (`SkeletalMeshComponent.GetAnimInstance` _turret)))
    (bind _returnvalue_2 (* (`KismetMathLibrary.GetRightVector` (`KismetMathLibrary.TransformRotation` (`SceneComponent.K2_GetComponentToWorld` _turret) (`/Game/DHLib/Misc/Turret/Covy_Defender_AnimBP.turret_rotation` _ascovy_defender_anim_bp))) (* (`self.MuzzleVelocity`) -1.0)))
    (`self.FireProjectile` (`KismetMathLibrary.MakeTransform` (`SceneComponent.K2_GetComponentLocation` (`self.ProjectileStart`))) _returnvalue_2)
    (`self.FireParticleSystem` _returnvalue_2)))

(fn `UserConstructionScript`)