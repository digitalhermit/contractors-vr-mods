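; Gravity hammer VR weapon, a grippable melee blade whose trigger unleashes a gravity slam while a second hand holds it.
; A cooldown-gated server hit multicasts a pivot spin, stopped on release, low elevation or timeout.
; The hit launches overlapping characters and spawns VictimHandlers to kill all but the wielder, while other actors take impulses and radial damage.
; Server-to-multicast events play hit, melee and drop sounds.
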(event `self.ReceiveBeginPlay`
  ;[1 1 1] Initialization
  (`parent.ReceiveBeginPlay`)
  (`MovementComponent.SetUpdatedComponent` (`self.HammerRotatingMovement`) (`self.ThrowableMesh`)))

(event `self.ReceiveTick`
  (params (DeltaSeconds :type "Float (single-precision)"))
  (bind (_hitfloorsnapshot_x _hitfloorsnapshot_y _hitfloorsnapshot_z) (`KismetMathLibrary.BreakVector` (`self.HitFloorSnapshot`)))
  (bind (_returnvalue_x _returnvalue_y _returnvalue_z) (`KismetMathLibrary.BreakVector` (`SceneComponent.K2_GetComponentLocation` (`self.HitDirection`))))
  (bind _returnvalue (- _returnvalue_z _hitfloorsnapshot_z))
  ;[1 1 1] Tick
  (`self.HandleAirborne`)
  (if (`self.GravityOn`)
    (`KismetSystemLibrary.PrintString` (`KismetStringLibrary.Concat_StrStr` "Elevation: " (`KismetStringLibrary.Conv_DoubleToString` _returnvalue)))
    (if (or (< _returnvalue 30.0) (> (- (`KismetSystemLibrary.GetGameTimeInSeconds`) (`self.TimeLastTriggered`)) (`self.HammerMaxActive`)))
      (`self.StopHammer`))
    (else
      (`self.StopHammer`))))

(event `ServerHandleHit`
  ;[1 1 1] Handle Multicasting Swing/Hit Information
  (bind _ready (`self.Hammer Ready`))
  (if _ready
    (set `self.TimeLastTriggered` (`KismetSystemLibrary.GetGameTimeInSeconds`))
    (set `self.GravityOn` true)
    (`self.MCHandleHit`)
    (`self.ServerPlaySoundAtLocation` "/Game/DHLib/Weapons/GHammer/Sounds/GHammerHit.GHammerHit" (`SceneComponent.K2_GetComponentLocation` (`self.ZomboyBlade`)))
    (`self.Apply Hit Effect`)
    (bind (_victims _otherhits) (`self.Select Victims`))
    (`self.Launch Characters` _victims)
    (`self.MaybeImpulseOthers` _otherhits)
    (`self.Handle Radial Damage` _victims)
    (`self.Kill Characters` _victims)))

(event `MCHandleHit`
  (bind _hammerrotatingmovement (`self.HammerRotatingMovement`))
  ;[1 1 1] Handle Multicasting Swing/Hit Information
  (set `RotatingMovementComponent.PivotTranslation` (`self.HitFloorSnapshot`) _hammerrotatingmovement)
  (set `RotatingMovementComponent.RotationRate` (struct :`Pitch` 1200.0) _hammerrotatingmovement))

(event `self.ZomboyBlade.OnDealDamageDelegate`
  (params (DamageLocation :type "Vector Structure"))
  ;[1 1 1] Melee sound triggered on dealing damage to other players (without gravity engaged)
  (if (not (`self.GravityOn`))
    (`self.ServerPlaySoundAtLocation` "/Game/DHLib/Weapons/GHammer/Sounds/GHammerMelee.GHammerMelee" DamageLocation))
  (`GameplayStatics.SpawnEmitterAtLocation` "/Game/ThirdPartyResources/Models/MilitaryWeapSilver/FX/P_Impact_Metal_Medium_Mobile.P_Impact_Metal_Medium_Mobile" DamageLocation))

(event `self.GripComponent.OnTriggerPressedEvent`
  (params (MotionController :type "ZomboyMotionControllerComponent Object Reference"))
  ;[1 1 1] Handle Gravity Hammer Engaged
  (if (`self.GravityTriggerReady`)
    (`ZomboyMotionControllerComponent.PlayHapticFeedback` MotionController "/Game/Core/VRInteractables/IndicateGrippedHaptic.IndicateGrippedHaptic")
    (set `self.HitFloorSnapshot` (`SceneComponent.RelativeLocation` (`self.HitPivot`)))
    (`self.ServerHandleHit`)))

(event `self.GripComponent.OnTriggerReleasedEvent`
  (params (MotionController :type "ZomboyMotionControllerComponent Object Reference"))
  ;[1 1 1] Handle Gravity Hammer Engaged
  (set `RotatingMovementComponent.RotationRate` (struct) (`self.HammerRotatingMovement`))
  (set `self.GravityOn` false))

(event `self.GripComponent1.OnHandInteractionBeginEvent`
  (params (Interaction :type "Interaction Structure (by ref)"))
  ;[1 1 1] Handle Gravity Hammer Engaged
  (set `self.GravityTriggerReady` true))

(event `self.GripComponent1.OnHandInteractionEndEvent`
  (params (Interaction :type "Interaction Structure (by ref)"))
  ;[1 1 1] Handle Gravity Hammer Engaged
  (set `self.GravityTriggerReady` false))

(event `self.OnGrabbed`
  (params (PrevState :type "InteractibleState Structure (by ref)") (CurrentState :type "InteractibleState Structure (by ref)"))
  ;[1 1 1] Dropping
  (`/Engine/EditorBlueprintResources/ActorMacros.Switch Has Authority`
    (:`Authority`
      (set `self.IsDropped` false))))

(event `self.OnDropped`
  (params (Location :type "Vector Structure (by ref)") (Velocity :type "Vector Structure (by ref)") (PrevState :type "InteractibleState Structure (by ref)") (CurrentState :type "InteractibleState Structure (by ref)"))
  ;[1 1 1] Dropping
  (`/Engine/EditorBlueprintResources/ActorMacros.Switch Has Authority`
    (:`Authority`
      (`self.StopHammer`)
      (set `self.IsDropped` true))))

(event `ServerPlaySoundAtLocation`
  (params (Sound :type "SoundBase Object Reference") (Location :type "Vector Structure"))
  ;[1 1 1] Play Sound
  (`self.MCPlaySound` Sound Location))

(event `self.ThrowableMesh.OnComponentHit`
  (params (HitComponent :type "PrimitiveComponent Object Reference") (OtherActor :type "Actor Object Reference") (OtherComp :type "PrimitiveComponent Object Reference") (NormalImpulse :type "Vector Structure") (Hit :type "HitResult Structure (by ref)"))
  ;[1 1 1] Drop sound when we hit something after being dropped
  (`/Engine/EditorBlueprintResources/ActorMacros.Switch Has Authority`
    (:`Authority`
      (if (`self.IsDropped`)
        (set `self.IsDropped` false)
        (`self.ServerPlaySoundAtLocation` "/Game/DHLib/Weapons/GHammer/Sounds/GHammerDrop.GHammerDrop" (`.Location` (`GameplayStatics.BreakHitResult` Hit)))))))

(event `MCPlaySound`
  (params (Sound :type "SoundBase Object Reference") (Location :type "Vector Structure"))
  ;[1 1 1] Play Sound
  (`GameplayStatics.PlaySoundAtLocation` Sound Location (struct) 1.0 1.0 0.0 "/Game/DHLib/Weapons/GHammer/Sounds/GHammerAttenuate.GHammerAttenuate" null null))

(fn `Apply Hit Effect`
  (bind _hitdirection (`self.HitDirection`))
  (bind (_returnvalue_location _returnvalue_rotation) (`KismetMathLibrary.BreakTransform` (`SceneComponent.K2_GetComponentToWorld` _hitdirection)))
  (bind _returnvalue (`|SpawnActorFromClass` "/Game/DHLib/Weapons/GHammer/GhamHitEffect.GhamHitEffect_C" (`KismetMathLibrary.MakeTransform` (+ _returnvalue_location (* (`SceneComponent.GetForwardVector` _hitdirection) 100.0)) _returnvalue_rotation) "AlwaysSpawn" "OverrideRootScale" null null))
  (set `self.HitEffect` _returnvalue)
  (`KismetSystemLibrary.PrintString` "HitEffect")
  (return))

(fn `CanBeginInteraction`
  (params (InteractionComponent :type "ZomboyInteractionComponent Object Reference") (MotionController :type "ZomboyMotionControllerComponent Object Reference"))
  (returns (ReturnValue :type Boolean))
  (bind _returnvalue (`parent.CanBeginInteraction` InteractionComponent MotionController))
  (if (== InteractionComponent (`self.GripComponent1`))
    (return (and _returnvalue (`ZomboyInteractionComponent.IsInteracting` (`self.GripComponent`))))
    (else
      (return _returnvalue))))

(fn `Hammer Ready`
  (returns (ready :type Boolean))
  (return (> (- (`KismetSystemLibrary.GetGameTimeInSeconds`) (`self.TimeLastTriggered`)) (`self.HammerDelay`))))

(fn `Handle Radial Damage`
  (params (Ignored :type "Array of Character Object Reference"))
  (bind _returnvalue (`self.GetOwnerPawn`))
  (bind _avoidradialdamage (`self.AvoidRadialDamage`))
  (bind _hitdirection (`self.HitDirection`))
  (bind _returnvalue_location (`KismetMathLibrary.BreakTransform` (`SceneComponent.K2_GetComponentToWorld` _hitdirection)))
  (`BlueprintSetLibrary.Set_AddItems` _avoidradialdamage Ignored)
  (bind _ascharacter (cast `Character` _returnvalue))
  (`BlueprintSetLibrary.Set_AddItems` _avoidradialdamage (`|MakeArray` _ascharacter))
  (bind _result (`BlueprintSetLibrary.Set_ToArray` _avoidradialdamage))
  (`GameplayStatics.ApplyRadialDamage` 200.0 (+ _returnvalue_location (* (`SceneComponent.GetForwardVector` _hitdirection) 200.0)) 300.0 null _result self (`ZomboyBlueprintLibrary.GetOwningController` _returnvalue) true) ; Damage everything but the Characters (example doors...)
  (return))

(fn `HandleAirborne`
  (`/Engine/EditorBlueprintResources/ActorMacros.Switch Has Authority`
    (:`Authority`
      (if (and (`self.OwnerAirborne`) (< (`KismetMathLibrary.VSize` (`self.GetVelocity` (`self.GetOwner`))) 20.0))
        (set `self.OwnerAirborne` false)
        (return)
        (else
          _)))
    (:`Remote`
      _))
  (return))

(fn `HandleDropping`
  (`/Engine/EditorBlueprintResources/ActorMacros.Switch Has Authority`
    (:`Authority`
      (if (and (`self.IsDropped`) (< (`KismetMathLibrary.VSize` (`self.GetVelocity`)) 0.1))
        (set `self.IsDropped` false)
        (return)
        (else
          (return))))
    (:`Remote`
      (return))))

(fn `Kill Characters`
  (params (Characters :type "Array of Character Object Reference"))
  (bind _returnvalue (`self.GetOwnerPawn`))
  (for _array_element Characters
    (if (!= _array_element _returnvalue)
      (`KismetSystemLibrary.PrintString` "Killing Character")
      (`|SpawnActorFromClass` "/Game/DHLib/Weapons/GHammer/VictimHandler.VictimHandler_C" (`self.GetTransform`) "AlwaysSpawn" "OverrideRootScale" null _array_element self (`ZomboyBlueprintLibrary.GetOwningController` _returnvalue) (`self.VictimDeathMaxDelay`) _returnvalue)
      (else
        (set `self.OwnerAirborne` true)))
    (return))
  (return))

(fn `Launch Characters`
  (params (Characters :type "Array of Character Object Reference"))
  (bind _launchvelocity (`self.LaunchVelocity`))
  (for _array_element Characters
    (bind _returnvalue (- (`SceneComponent.K2_GetComponentLocation` (`Character.CapsuleComponent` _array_element)) (`SceneComponent.K2_GetComponentLocation` (`self.HitDirection`))))
    (bind _returnvalue_2 (/ _returnvalue (`KismetMathLibrary.VSize` _returnvalue)))
    (bind (_returnvalue_x _returnvalue_y _returnvalue_z) (`KismetMathLibrary.BreakVector` (* _returnvalue_2 _launchvelocity)))
    (`Character.LaunchCharacter` _array_element (`KismetMathLibrary.MakeVector` _returnvalue_x _returnvalue_y (`KismetMathLibrary.FClamp` (`KismetMathLibrary.Abs` _returnvalue_z) (/ _launchvelocity 3.0) _launchvelocity)) false false)
    (`KismetSystemLibrary.PrintString` (`KismetStringLibrary.Concat_StrStr` "Launch Character: " (`KismetStringLibrary.Conv_VectorToString` _returnvalue_2)))
    (return))
  (return))

(fn `MaybeImpulseOthers`
  (params (Others :type "Array of Actor Object Reference"))
  (for _array_element Others
    (bind _rootcomponent (`Actor.RootComponent` _array_element))
    (bind _asprimitive_component (cast `PrimitiveComponent` _rootcomponent))
    (if (`SceneComponent.IsSimulatingPhysics` _rootcomponent "None")
      (bind (_returnvalue_x _returnvalue_y _returnvalue_z) (`KismetMathLibrary.BreakVector` (* (/ (- (`SceneComponent.K2_GetComponentLocation` _rootcomponent) (`SceneComponent.K2_GetComponentLocation` (`self.HitDirection`))) 1.0) (`self.LaunchVelocity`))))
      (`PrimitiveComponent.AddImpulse` _asprimitive_component (`KismetMathLibrary.MakeVector` _returnvalue_x _returnvalue_y (`KismetMathLibrary.Abs` _returnvalue_z)) "None" false)
      (`KismetSystemLibrary.PrintString` "Impulse")))
  (return))

(fn `Select Victims`
  (returns (Victims :type "Array of Character Object Reference") (OtherHits :type "Array of Actor Object Reference"))
  (`BlueprintSetLibrary.Set_Clear` (`self.Victims`))
  (`BlueprintSetLibrary.Set_Clear` (`self.OtherHits`))
  (for _array_element (`PrimitiveComponent.GetOverlappingActors` (`self.SplashDamageCollision`) null)
    (bind _ascharacter (cast `Character` _array_element)
      (:`then`
        (if (or (!= _ascharacter (`self.GetOwnerPawn`)) (and (`self.LaunchOwnerOnHit`) (not (`self.OwnerAirborne`))))
          (`BlueprintSetLibrary.Set_Add` (`self.Victims`) _ascharacter)))
      (:`CastFailed`
        (`BlueprintSetLibrary.Set_Add` (`self.OtherHits`) _array_element))))
  (bind _result (`BlueprintSetLibrary.Set_ToArray` (`self.Victims`)))
  (bind _result_2 (`BlueprintSetLibrary.Set_ToArray` (`self.OtherHits`)))
  (return _result _result_2))

(fn `StopHammer`
  (bind _hammerrotatingmovement (`self.HammerRotatingMovement`))
  (`MovementComponent.StopMovementImmediately` _hammerrotatingmovement)
  (set `RotatingMovementComponent.RotationRate` (struct) _hammerrotatingmovement)
  (set `self.GravityOn` false)
  (return))

(fn `UserConstructionScript`
  (`parent.UserConstructionScript`))