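; Automated turret actor that acquires pawns entering its sphere scanner and fires projectiles at them.
; The Covy_Defender anim Blueprint receives target enter and exit events and supplies the fire flag and aim rotation, which Tick uses for rate-limited shots.
; Each shot resets a particle system that reports particle data back to the actor, which sphere-traces along particle velocity and applies explosion damage to hits.
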(event `self.ReceiveBeginPlay`
  (set `self.LastFireTime` 0.0)
  (`NiagaraComponent.SetVariableObject` (`self.Projectile`) "BPCallback" self))

(event `self.ReceiveTick`
  (params (DeltaSeconds :type "Float (single-precision)"))
  (bind _ascovy_defender_anim_bp (cast `/TestG/Misc/Turret/Covy_Defender_AnimBP` (`SkeletalMeshComponent.GetAnimInstance` (`self.Turret`))))
  (if (`/TestG/Misc/Turret/Covy_Defender_AnimBP.fire_at_target` _ascovy_defender_anim_bp)
    (`self.MaybeFire`)))

(event `self.SphereScanner.OnComponentBeginOverlap`
  (params (OverlappedComponent :type "PrimitiveComponent Object Reference") (OtherActor :type "Actor Object Reference") (OtherComp :type "PrimitiveComponent Object Reference") (OtherBodyIndex :type Integer) (bFromSweep :type Boolean) (SweepResult :type "HitResult Structure (by ref)"))
  (bind _aspawn (cast `Pawn` OtherActor))
  (bind _ascovy_defender_anim_bp (cast `/TestG/Misc/Turret/Covy_Defender_AnimBP` (`SkeletalMeshComponent.GetAnimInstance` (`self.Turret`))))
  (`/TestG/Misc/Turret/Covy_Defender_AnimBP.TargetAcquired` _ascovy_defender_anim_bp _aspawn))

(event `self.SphereScanner.OnComponentEndOverlap`
  (params (OverlappedComponent :type "PrimitiveComponent Object Reference") (OtherActor :type "Actor Object Reference") (OtherComp :type "PrimitiveComponent Object Reference") (OtherBodyIndex :type Integer))
  (bind _aspawn (cast `Pawn` OtherActor))
  (bind _ascovy_defender_anim_bp (cast `/TestG/Misc/Turret/Covy_Defender_AnimBP` (`SkeletalMeshComponent.GetAnimInstance` (`self.Turret`))))
  (`/TestG/Misc/Turret/Covy_Defender_AnimBP.TargetOutOfRange` _ascovy_defender_anim_bp _aspawn))

(event `self.ReceiveParticleData`
  (params (Data :type "Array of BasicParticleData Structure (by ref)") (NiagaraSystem :type "NiagaraSystem Object Reference"))
  (for _array_element Data
    (bind (_position _size _velocity) (break `BasicParticleData` _array_element))
    (bind _outhit (`KismetSystemLibrary.SphereTraceSingleForObjects` _position (+ _position (* _velocity 0.1)) _size (`self.ObjectTypesArray`)))
    (`self.ProjectileDamage` (`.HitActor` (`GameplayStatics.BreakHitResult` _outhit)))))

(event `ProjectileDamage`
  (params (DamagedActor :type "Actor Object Reference"))
  (if (`KismetSystemLibrary.IsValid` DamagedActor)
    (`GameplayStatics.ApplyDamage` DamagedActor 30.0 (`self.GetInstigatorController` DamagedActor) DamagedActor "/Game/Core/VRInteractables/Throwables/Grenades/ExplosionDamageType.ExplosionDamageType_C")
    (`KismetSystemLibrary.PrintString` (`KismetStringLibrary.Concat_StrStr` "Hit" (`KismetSystemLibrary.GetPathName` DamagedActor)))))

(event `SRVPlaySoundOnAll`
  (params (Audio :type "AudioComponent Object Reference"))
  (`self.MCPlaySound` Audio))

(event `MCPlaySound`
  (params (Audio :type "AudioComponent Object Reference"))
  (`AudioComponent.Play` Audio 0.0))

(fn `MaybeFire`
  (bind _returnvalue (`KismetSystemLibrary.GetGameTimeInSeconds`))
  (bind _turret (`self.Turret`))
  (bind _projectile (`self.Projectile`))
  (if (> (- _returnvalue (`self.LastFireTime`)) 0.5)
    (set `self.LastFireTime` _returnvalue)
    (bind _ascovy_defender_anim_bp (cast `/TestG/Misc/Turret/Covy_Defender_AnimBP` (`SkeletalMeshComponent.GetAnimInstance` _turret)))
    (`KismetSystemLibrary.PrintString` "FIRE!!!!")
    (`NiagaraComponent.SetVariableVec3` _projectile "Velocity" (* (`KismetMathLibrary.GetRightVector` (`KismetMathLibrary.TransformRotation` (`SceneComponent.K2_GetComponentToWorld` _turret) (`/TestG/Misc/Turret/Covy_Defender_AnimBP.turret_rotation` _ascovy_defender_anim_bp))) -5000.0))
    (`NiagaraComponent.ResetSystem` _projectile)
    (`self.MCPlaySound` (`self.TurretBlast`))))

(fn `UserConstructionScript`)